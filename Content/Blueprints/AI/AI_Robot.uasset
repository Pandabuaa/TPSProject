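; AI robot that loops an idle animation montage while the third-person player character is inside its trigger sphere.
; Sphere overlap starts the montage and a timer set to its returned length to replay it.
; Leaving the sphere clears that timer.
; A random navmesh wander event exists, but the nodes that would start it are disconnected, so the robot does not roam.
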(event `self.ReceiveBeginPlay`)

(event `AI_Move`
  (`|AIMoveTo` self (`NavigationSystemV1.K2_GetRandomLocationInNavigableRadius` (`self.K2_GetActorLocation`) 5000.0 null null) null 100.0))

(event `loop`
  (bind _returnvalue (`AnimInstance.Montage_Play` (`SkeletalMeshComponent.GetAnimInstance` (`self.Mesh`)) "/Game/Blueprints/AI/A_idle_01_Montage.A_idle_01_Montage" 1.0 "MontageLength" 0.0 true :!label _label))
  (bind _returnvalue_2 (`KismetSystemLibrary.K2_SetTimerDelegate` (delegate `loop`) _returnvalue true)))

(event `self.Sphere.OnComponentBeginOverlap`
  (params (OverlappedComponent :type "PrimitiveComponent Object Reference") (OtherActor :type "Actor Object Reference") (OtherComp :type "PrimitiveComponent Object Reference") (OtherBodyIndex :type Integer) (bFromSweep :type Boolean) (SweepResult :type "HitResult Structure (by ref)"))
  (cast `/Game/ThirdPersonCPP/Blueprints/ThirdPersonCharacter` OtherActor)
  (goto _label))

(event `self.Sphere.OnComponentEndOverlap`
  (params (OverlappedComponent :type "PrimitiveComponent Object Reference") (OtherActor :type "Actor Object Reference") (OtherComp :type "PrimitiveComponent Object Reference") (OtherBodyIndex :type Integer))
  (cast `/Game/ThirdPersonCPP/Blueprints/ThirdPersonCharacter` OtherActor)
  (`KismetSystemLibrary.K2_ClearAndInvalidateTimerHandle` (stale `loop` _returnvalue_2)))

(fn `UserConstructionScript`)